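; BP_Complete_scenter is a completion indicator that reacts on Tick to its CountHits value, which is not changed in this graph.
; Above zero, it shows Niagara, makes Cube1 glow and displays UI_Tutorial for five seconds, then forces garbage collection.
; Otherwise it hides the effect and restores the material.
; Two cross-resetting DoOnce gates make each response fire once per state change.
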(event EventBeginPlay
  (|CallParentFunction) ; This node is disabled and will not be called.\nDrag off pins to build functionality.
)

(event Collision|EventActorBeginOverlap
  (params (OtherActor :type Actor%20Object%20Reference)))

(event EventTick
  (params (DeltaSeconds :type Float%20%28single-precision%29))
  (bind _cube1 (Variables|Default|GetCube1))
  (if (> (Variables|Default|GetCountHits) 0)
    (Utilities|FlowControl|DoOnce false :!label _label
      (:Completed
        (Utilities|FlowControl|Sequence
          (:then_0
            (Rendering|SetVisibility (Variables|Default|GetNiagara) true false)
            (Rendering|Material|SetMaterial _cube1 0 "/Game/New_Game/Materials/GuestMeshes/MI_glow.MI_glow")
            (bind _returnvalue (UserInterface|CreateWidget "/Game/BluePrints/Widget/UI_Tutorial.UI_Tutorial_C"))
            (bind _output_get (Variables|Default|SetNewVar_0 _returnvalue))
            (UserInterface|Viewport|AddtoViewport _output_get 0)
            (Utilities|FlowControl|Delay 5.0)
            (Widget|RemovefromParent (Variables|Default|GetNewVar_0))
            (Variables|Default|SetNewVar_0 0)
            (Utilities|Platform|CollectGarbage))
          (:then_1
            (goto _label_2 Reset)))))
    (else
      (Utilities|FlowControl|DoOnce false :!label _label_2
        (:Completed
          (Rendering|SetVisibility (Variables|Default|GetNiagara) false false)
          (Rendering|Material|SetMaterial _cube1 0 (Variables|Default|GetMaterial))
          (goto _label Reset))))))

(fn ConstructionScript
  (|CallParentFunction))