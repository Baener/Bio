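; BP_EndCrystal is an end crystal actor that reveals an effect and spawns a final trigger once its hit counter reaches zero.
; Tick polls CountHits, which this graph does not decrement, and sets it to -1 at zero so the sequence does not repeat every frame.
; It then makes the Niagara1 component visible and spawns BP_FinalTrigger at that component's world location.
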(event EventBeginPlay
  (|CallParentFunction) ; This node is disabled and will not be called.\nDrag off pins to build functionality.
)

(event Collision|EventActorBeginOverlap
  (params (OtherActor :type Actor%20Object%20Reference)))

(event EventTick
  (params (DeltaSeconds :type Float%20%28single-precision%29))
  (if (== (Variables|Default|GetCountHits) 0)
    (Variables|Default|SetCountHits -1)
    (Rendering|SetVisibility (Variables|Default|GetNiagara1) true false)
    (Game|SpawnActorfromClass "/Game/BluePrints/BP_FinalTrigger.BP_FinalTrigger_C" (Math|Transform|MakeTransform (Transformation|GetWorldLocation (Variables|Default|GetNiagara1)) "0, 0, 0" "1.000000,1.000000,1.000000") "Undefined" "MultiplyWithRoot" 0 0)))

(fn ConstructionScript
  (|CallParentFunction))