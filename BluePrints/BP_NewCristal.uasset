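; Puzzle crystal that emits a Niagara beam while hit by other beams, chaining activation from crystal to crystal.
; CountHits tracks incoming beams; OnNiagara toggles beam and sounds, then line-traces forward to adjust the next crystal's count and recursively call its OnNiagara.
; With the player in the trigger zone, E or Q rotates an active crystal by timeline, releasing the old target, updating beam length and powering the new target on finish.
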(event OnComponentBeginOverlap(TriggerZone)
  (params (OverlappedComponent :type Primitive%20Component%20Object%20Reference) (OtherActor :type Actor%20Object%20Reference) (OtherComp :type Primitive%20Component%20Object%20Reference) (OtherBodyIndex :type Integer) (bFromSweep :type Boolean) (SweepResult :type Hit%20Result%20Structure%20%28by%20ref%29))
  ;[1 1 1] Check Player in overlap
  (Utilities|Casting|CastToBP_DemoThirdPersonCharacter OtherActor)
  (Variables|Default|SetCheckPlayer true))

(event OnComponentEndOverlap(TriggerZone)
  (params (OverlappedComponent :type Primitive%20Component%20Object%20Reference) (OtherActor :type Actor%20Object%20Reference) (OtherComp :type Primitive%20Component%20Object%20Reference) (OtherBodyIndex :type Integer))
  ;[1 1 1] Check Player in overlap
  (Utilities|Casting|CastToBP_DemoThirdPersonCharacter OtherActor)
  (Variables|Default|SetCheckPlayer false))

(event Custom|OnNiagara
  (bind _cube1 (Variables|Default|GetCube1))
  (bind _cube1_2 (Variables|Default|GetCube1))
  (bind _returnvalue (Transformation|GetWorldLocation _cube1_2))
  (bind _returnvalue_2 (Transformation|GetWorldLocation _cube1))
  ;[1 1 1] Checks Counter beams and Visible Niagara
  (if (> (Variables|Default|GetCountHits) 0)
    (if (not (Rendering|IsVisible (Variables|Default|GetNiagara)))
      ;[1 1 1] Set Active and Activate Niagara
      (Variables|Default|SetActive true)
      (Rendering|SetVisibility (Variables|Default|GetNiagara) true false)
      ;[1 1 1] Sound
      (Audio|Components|Audio|Play (Variables|Default|GetSwitchOn) 0.0)
      (Audio|Components|Audio|Play (Variables|Default|GetEnabling) 0.0)
      ;[1 1 1] Line Trace for Next Cristal
      (bind _outhit (Collision|LineTraceForObjects _returnvalue (+ _returnvalue (* (Math|Vector|GetForwardVector _cube1_2) (Variables|Default|GetRangeBeam))) (Utilities|Array|MakeArray "ObjectTypeQuery2" "ObjectTypeQuery1") false 0 "None"))
      ;[1 1 1] Set Range Niagara and Increase Counter Beams and Call Event On_Niagara
      (Niagara|SetNiagaraVariable(Vector3) (Variables|Default|GetNiagara) "User.End" (Math|Vector|MakeVector (.Distance (Collision|BreakHitResult _outhit)) 0.0 0.0))
      (bind _asbp_new_cristal (Utilities|Casting|CastToBP_NewCristal (.HitActor (Collision|BreakHitResult _outhit))))
      (Variables|BP_NewCristal_C|SetCountHits _asbp_new_cristal (+ (Variables|BP_NewCristal_C|GetCountHits _asbp_new_cristal) 1))
      (CallFunction|OnNiagara _asbp_new_cristal))
    (elif (Rendering|IsVisible (Variables|Default|GetNiagara))
      ;[1 1 1] Set Deactive and Deactivate Niagara
      (Variables|Default|SetActive false)
      (Rendering|SetVisibility (Variables|Default|GetNiagara) false false)
      ;[1 1 1] StopSound
      (Audio|Components|Audio|Stop (Variables|Default|GetEnabling))
      ;[1 1 1] Line Trace for Next Cristal
      (bind _outhit_2 (Collision|LineTraceForObjects _returnvalue_2 (+ _returnvalue_2 (* (Math|Vector|GetForwardVector _cube1) (Variables|Default|GetRangeBeam))) (Utilities|Array|MakeArray "ObjectTypeQuery2" "ObjectTypeQuery1") false 0 "None"))
      ;[1 1 1] Check Active Niagara for Next Cristall and Decrease Counter Beams and Call On_Niagara
      (bind _asbp_new_cristal_2 (Utilities|Casting|CastToBP_NewCristal (.HitActor (Collision|BreakHitResult _outhit_2))))
      (Variables|BP_NewCristal_C|SetCountHits _asbp_new_cristal_2 (- (Variables|BP_NewCristal_C|GetCountHits _asbp_new_cristal_2) 1))
      (CallFunction|OnNiagara _asbp_new_cristal_2))))

(event EventBeginPlay
  ;[1 1 1] BeingPlay Set Angle And Call Event On Niagara
  (Variables|Default|SetAngle (.yaw (Variables|/Script/Engine.SceneComponent|GetRelativeRotation (Variables|Default|GetCube1))))
  (CallFunction|OnNiagara))

(event Input|KeyboardEvents|E
  (params (Key :type Key%20Structure))
  (bind _cube1 (Variables|Default|GetCube1))
  (bind _cube1_2 (Variables|Default|GetCube1))
  (bind _cube1_3 (Variables|Default|GetCube1))
  (bind _returnvalue (Transformation|GetWorldLocation _cube1_3))
  (bind _returnvalue_2 (Transformation|GetWorldLocation _cube1))
  (bind _returnvalue_3 (Transformation|GetWorldLocation _cube1_2))
  ;[1 1 1] Pressed E or Q and Checks
  (:Pressed
    (if (Variables|Default|GetCanRotate)
      (Variables|Default|SetAngleRotate (Variables|Default|GetRotate))
      (if (Variables|Default|GetCheckPlayer)
        (if (Variables|Default|GetActive)
          ;[1 1 1] Line Trace for Cristal Befor Rotate and Deactive Rotate
          (Variables|Default|SetCanRotate false)
          (bind _outhit (Collision|LineTraceForObjects _returnvalue_2 (+ _returnvalue_2 (* (Math|Vector|GetForwardVector _cube1) (Variables|Default|GetRangeBeam))) (Utilities|Array|MakeArray "ObjectTypeQuery2" "ObjectTypeQuery1") false 0 "None"))
          ;[1 1 1] Decrease Counter for Cristal Before Rotate and call him On_Niagara
          (bind _asbp_new_cristal (Utilities|Casting|CastToBP_NewCristal (.HitActor (Collision|BreakHitResult _outhit)))
            (:then
              (Variables|BP_NewCristal_C|SetCountHits _asbp_new_cristal (- (Variables|BP_NewCristal_C|GetCountHits _asbp_new_cristal) 1))
              (CallFunction|OnNiagara _asbp_new_cristal)
              ;[1 1 1] Rotate Cristal
              (bind _rotator (Timeline|Timeline PlayFromStart)
                (:Update
                  (Transformation|SetRelativeRotation (Variables|Default|GetCube1) (Math|Rotator|MakeRotator 0.0 0.0 (+ (* (Variables|Default|GetAngleRotate) _rotator) (Variables|Default|GetAngle))) false false)
                  ;[1 1 1] Line Trace for Objects and Change Distance for Cristal
                  (bind _outhit_2 (Collision|LineTraceForObjects _returnvalue_3 (+ _returnvalue_3 (* (Math|Vector|GetForwardVector _cube1_2) (Variables|Default|GetRangeBeam))) (Utilities|Array|MakeArray "ObjectTypeQuery2" "ObjectTypeQuery1") false 0 "None" true "(R=1.000000,G=0.000000,B=0.741744,A=1.000000)"))
                  (Niagara|SetNiagaraVariable(Vector3) (Variables|Default|GetNiagara) "User.End" (Math|Vector|MakeVector (.Distance (Collision|BreakHitResult _outhit_2)) 0.0 0.0)))
                (:Finished
                  (Variables|Default|SetCanRotate true)
                  (Variables|Default|SetAngle (+ (Variables|Default|GetAngle) (Variables|Default|GetAngleRotate)))
                  ;[1 1 1] Line Trace for Next Cristal
                  (bind _outhit_3 (Collision|LineTraceForObjects _returnvalue (+ _returnvalue (* (Math|Vector|GetForwardVector _cube1_3) (Variables|Default|GetRangeBeam))) (Utilities|Array|MakeArray "ObjectTypeQuery2" "ObjectTypeQuery1") false 0 "None"))
                  ;[1 1 1] Increase Counter for Next Cristal and Call him On_Niagara
                  (if (Variables|Default|GetActive)
                    (Niagara|SetNiagaraVariable(Vector3) (Variables|Default|GetNiagara) "User.End" (Math|Vector|MakeVector (+ (.Distance (Collision|BreakHitResult _outhit_3)) 25.0) 0.0 0.0))
                    (bind _asbp_new_cristal_2 (Utilities|Casting|CastToBP_NewCristal (.HitActor (Collision|BreakHitResult _outhit_3))))
                    (Variables|BP_NewCristal_C|SetCountHits _asbp_new_cristal_2 (+ (Variables|BP_NewCristal_C|GetCountHits _asbp_new_cristal_2) 1))
                    (CallFunction|OnNiagara _asbp_new_cristal_2)))))
            (:CastFailed
              (Timeline|Timeline PlayFromStart))))))))

(event Input|KeyboardEvents|Q
  (params (Key :type Key%20Structure))
  (bind _cube1 (Variables|Default|GetCube1))
  (bind _cube1_2 (Variables|Default|GetCube1))
  (bind _cube1_3 (Variables|Default|GetCube1))
  (bind _returnvalue (Transformation|GetWorldLocation _cube1_3))
  (bind _returnvalue_2 (Transformation|GetWorldLocation _cube1))
  (bind _returnvalue_3 (Transformation|GetWorldLocation _cube1_2))
  ;[1 1 1] Pressed E or Q and Checks
  (:Pressed
    (if (Variables|Default|GetCanRotate)
      (Variables|Default|SetAngleRotate (* (Variables|Default|GetRotate) -1.0))
      (if (Variables|Default|GetCheckPlayer)
        (if (Variables|Default|GetActive)
          ;[1 1 1] Line Trace for Cristal Befor Rotate and Deactive Rotate
          (Variables|Default|SetCanRotate false)
          (bind _outhit (Collision|LineTraceForObjects _returnvalue_2 (+ _returnvalue_2 (* (Math|Vector|GetForwardVector _cube1) (Variables|Default|GetRangeBeam))) (Utilities|Array|MakeArray "ObjectTypeQuery2" "ObjectTypeQuery1") false 0 "None"))
          ;[1 1 1] Decrease Counter for Cristal Before Rotate and call him On_Niagara
          (bind _asbp_new_cristal (Utilities|Casting|CastToBP_NewCristal (.HitActor (Collision|BreakHitResult _outhit)))
            (:then
              (Variables|BP_NewCristal_C|SetCountHits _asbp_new_cristal (- (Variables|BP_NewCristal_C|GetCountHits _asbp_new_cristal) 1))
              (CallFunction|OnNiagara _asbp_new_cristal)
              ;[1 1 1] Rotate Cristal
              (bind _rotator (Timeline|Timeline PlayFromStart)
                (:Update
                  (Transformation|SetRelativeRotation (Variables|Default|GetCube1) (Math|Rotator|MakeRotator 0.0 0.0 (+ (* (Variables|Default|GetAngleRotate) _rotator) (Variables|Default|GetAngle))) false false)
                  ;[1 1 1] Line Trace for Objects and Change Distance for Cristal
                  (bind _outhit_2 (Collision|LineTraceForObjects _returnvalue_3 (+ _returnvalue_3 (* (Math|Vector|GetForwardVector _cube1_2) (Variables|Default|GetRangeBeam))) (Utilities|Array|MakeArray "ObjectTypeQuery2" "ObjectTypeQuery1") false 0 "None" true "(R=1.000000,G=0.000000,B=0.741744,A=1.000000)"))
                  (Niagara|SetNiagaraVariable(Vector3) (Variables|Default|GetNiagara) "User.End" (Math|Vector|MakeVector (.Distance (Collision|BreakHitResult _outhit_2)) 0.0 0.0)))
                (:Finished
                  (Variables|Default|SetCanRotate true)
                  (Variables|Default|SetAngle (+ (Variables|Default|GetAngle) (Variables|Default|GetAngleRotate)))
                  ;[1 1 1] Line Trace for Next Cristal
                  (bind _outhit_3 (Collision|LineTraceForObjects _returnvalue (+ _returnvalue (* (Math|Vector|GetForwardVector _cube1_3) (Variables|Default|GetRangeBeam))) (Utilities|Array|MakeArray "ObjectTypeQuery2" "ObjectTypeQuery1") false 0 "None"))
                  ;[1 1 1] Increase Counter for Next Cristal and Call him On_Niagara
                  (if (Variables|Default|GetActive)
                    (Niagara|SetNiagaraVariable(Vector3) (Variables|Default|GetNiagara) "User.End" (Math|Vector|MakeVector (+ (.Distance (Collision|BreakHitResult _outhit_3)) 25.0) 0.0 0.0))
                    (bind _asbp_new_cristal_2 (Utilities|Casting|CastToBP_NewCristal (.HitActor (Collision|BreakHitResult _outhit_3))))
                    (Variables|BP_NewCristal_C|SetCountHits _asbp_new_cristal_2 (+ (Variables|BP_NewCristal_C|GetCountHits _asbp_new_cristal_2) 1))
                    (CallFunction|OnNiagara _asbp_new_cristal_2)))))
            (:CastFailed
              (Timeline|Timeline PlayFromStart))))))))

(fn ConstructionScript)